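; Church sequence actor that starts the windows sequence and reacts to its completion.
; Pressing X within 500 units (2D), at the matching narration count, moves GameObjectOne onto the player and flags the sequence active in GI_New, once only.
; Tick polls GI_New until at least three windows are fixed, then teleports GameObjectTwo onto the player a single time.
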(event `self.ReceiveBeginPlay`
  (bind _outactors (`GameplayStatics.GetAllActorsOfClass` "/Game/FirstPersonBP/Blueprints/FirstPersonCharacter.FirstPersonCharacter_C"))
  (set `self.Player` (`|GetArrayItem` _outactors)))

(event `self.ReceiveTick`
  (params (DeltaSeconds :type "Float (single-precision)"))
  (if (not (`self.isDone`))
    (bind _asgi_new (cast `/Game/Blueprints/GI_New` (`GameplayStatics.GetGameInstance`)))
    (if (>= (`/Game/Blueprints/GI_New.WindowsFixed` _asgi_new) 3)
      (`self.K2_SetActorLocation` (`self.GameObjectTwo`) (`self.K2_GetActorLocation` (`self.Player`)) false true)
      (set `self.isDone` true))))

(event `Key|X` :consume false
  (params (Key :type "Key Structure"))
  (:`Pressed`
    (if (< (`self.xCounter`) 1)
      (bind _asgi_new (cast `/Game/Blueprints/GI_New` (`GameplayStatics.GetGameInstance`)))
      (bind _isclose_ (`self.IsPlayerClose` (`self.Player`) self))
      (if (and _isclose_ (== (`/Game/Blueprints/GI_New.NarrationCounter` _asgi_new) (`self.NarrationNum`)))
        (bind _result (`/Engine/EditorBlueprintResources/StandardMacros.IncrementInt` (`self.xCounter`))
          (:`  `
            (set `self.xCounter` _result)
            (`self.K2_SetActorLocation` (`self.GameObjectOne`) (`self.K2_GetActorLocation` (`self.Player`)) false false)
            (set `/Game/Blueprints/GI_New.WindowsSequenceIsActive` true _asgi_new)))))))

(fn `IsPlayerClose`
  (params (GameObjectOne :type "Actor Object Reference") (GameObjectTwo :type "Actor Object Reference"))
  (returns (`isClose?` :type Boolean))
  (bind _returnvalue (<= (`KismetMathLibrary.Vector_Distance2D` (`self.K2_GetActorLocation` GameObjectOne) (`self.K2_GetActorLocation` GameObjectTwo)) 500.0))
  (if _returnvalue
    (return _returnvalue)))

(fn `UserConstructionScript`)