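; GI_New, apparently a Game Instance, holds game-flow state for intro, outro, cinematics, fades, game over and press-X prompts.
; ResetSelf restores the flags to their starting state with only IsIntro true, and ResetString restores the "Press X to Continue" prompt.
; NextNarration only prints NarrationCounter, as its increment is not wired to execute.
; PressX and FindClosestInteractableObject are empty stubs.
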(fn `FindClosestInteractableObject`
  (params (PlayerPos :type "Vector Structure") (Radius :type "Float (double-precision)")))

(fn `NextNarration`
  (`KismetSystemLibrary.PrintString` (`KismetStringLibrary.Conv_IntToString` (`self.NarrationCounter`))))

(fn `PressX`)

(fn `ResetSelf`
  (set `self.isIntro` true)
  (set `self.FadeToBlack` false)
  (set `self.isOutro` false)
  (set `self.IsAtEnd` false)
  (set `self.PressXToContinue` false)
  (set `self.isGameOver` false)
  (set `self.PressedX` false)
  (set `self.isClear` false)
  (set `self.PlayerStop` false)
  (set `self.StartFade` false)
  (set `self.IsInCine` false))

(fn `ResetString`
  (set `self.SwapString` "Press X to Continue"))